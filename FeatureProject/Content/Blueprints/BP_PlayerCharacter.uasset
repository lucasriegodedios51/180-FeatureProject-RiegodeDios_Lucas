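; Player character Blueprint that sets up the player's crosshair and a debug key for testing damage.
; On BeginPlay it caches the BP_PlayerController reference and, if that cast succeeds, adds a WBP_Crosshair widget to the viewport as an aiming reticle.
; Pressing 1 applies fixed damage to the character's own AC_HealthComponent and prints the remaining health, labeled "Enemy Health".
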(event `self.ReceiveBeginPlay`
  ; Allows for the controller to work when trying to control the player this also adds for a reticle to give some sort of visual as to where the player shoots
  (bind _asbp_player_controller (cast `/Game/Blueprints/BP_PlayerController` (`GameplayStatics.GetPlayerController` 0)))
  (set `self.PlayerControllerRef` _asbp_player_controller)
  (bind _returnvalue (`|CreateWidget` "/Game/UI/WBP_Crosshair.WBP_Crosshair_C"))
  (`UserWidget.AddToViewport` _returnvalue 0))

(event `Key|One`
  (params (Key :type "Key Structure"))
  (bind _returnvalue (`self.GetComponentByClass` "/Game/Blueprints/AC_HealthComponent.AC_HealthComponent_C"))
  ; Take Damage when 1 is pressed
  (:`Pressed`
    (`/Engine/EditorBlueprintResources/StandardMacros.IsValid` _returnvalue
      (:`Is Valid`
        (`/Game/Blueprints/AC_HealthComponent.Apply Damage` (`self.AC_HealthComponent`) 10.0)
        (`KismetSystemLibrary.PrintString` (`KismetStringLibrary.Concat_StrStr` "Enemy Health: " (`KismetStringLibrary.Conv_DoubleToString` (`/Game/Blueprints/AC_HealthComponent.CurrentHealth` _returnvalue))))))))

(fn `UserConstructionScript`)