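; AC_HealthComponent is an actor component that tracks health and a separate over-health shield pool.
; On BeginPlay it sets current health to the maximum, then damage and healing functions adjust it, clamped between zero and that maximum.
; AddOverHealth fills the shield up to its own cap, but ApplyDamage never draws from it.
; Both add functions print the new value to screen; no death handling is present.
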(event `self.ReceiveBeginPlay`
  (set `self.CurrentHealth` (`self.MaxHealth`)))

(fn `AddHealth`
  (params (Amount :type "Float (double-precision)"))
  (bind _output_get (set `self.CurrentHealth` (`KismetMathLibrary.FClamp` (+ Amount (`self.CurrentHealth`)) 0.0 (`self.MaxHealth`))))
  (`KismetSystemLibrary.PrintString` (`KismetStringLibrary.Concat_StrStr` "Player Health: " (`KismetStringLibrary.Conv_DoubleToString` _output_get))))

(fn `AddOverHealth`
  (params (Amount :type "Float (double-precision)" :default 50.0))
  (bind _output_get (set `self.OverHealth` (`KismetMathLibrary.FClamp` (+ (`self.OverHealth`) Amount) 0.0 (`self.MaxOverHeath`))))
  (`KismetSystemLibrary.PrintString` (`KismetStringLibrary.Concat_StrStr` "Shield: " (`KismetStringLibrary.Conv_DoubleToString` _output_get))))

(fn `Apply Damage`
  (params (Damage :type "Float (double-precision)"))
  (set `self.CurrentHealth` (`KismetMathLibrary.FClamp` (- (`self.CurrentHealth`) Damage) 0.0 (`self.MaxHealth`))))