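; Player controller that handles movement and projectile throwing (a hammer throw) for BP_PlayerCharacter.
; On BeginPlay it registers the IMC_Input Enhanced Input context and caches the player character.
; IA_Move feeds movement input along fixed world axes, independent of camera or actor facing.
; IA_Shoot spawns BP_Projectile at the character's FirePoint with the actor's rotation, gated by CanShoot, which a HammerCooldown timer resets.
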(event `self.ReceiveBeginPlay`
  (bind _returnvalue (subsystem `EnhancedInputLocalPlayerSubsystem`))
  ; Set Player as a refercnce
  (`/Engine/EditorBlueprintResources/StandardMacros.IsValid` _returnvalue
    (:`Is Valid`
      (`EnhancedInputSubsystemInterface.AddMappingContext` _returnvalue "/Game/Blueprints/Inputs/IMC_Input.IMC_Input" 0 (struct))
      (bind _asbp_player_character (cast `/Game/Blueprints/BP_PlayerCharacter` (`GameplayStatics.GetPlayerCharacter` 0)))
      (set `self.Player_Ref` _asbp_player_character))))

(event `EnhancedInput|/Game/Blueprints/Inputs/IA_Move`
  (params (ActionValue :type "Vector Structure") (ElapsedSeconds :type "Float (double-precision)") (TriggeredSeconds :type "Float (double-precision)") (InputAction :type "InputAction Object Reference" :default "/Game/Blueprints/Inputs/IA_Move.IA_Move"))
  (bind _player_ref (`self.Player_Ref`))
  ; Allow Player to move using wasd
  (:`Triggered`
    (`Pawn.AddMovementInput` _player_ref (0.0 1.0 0.0) ActionValue_X false)
    (`Pawn.AddMovementInput` _player_ref (1.0 0.0 0.0) ActionValue_Y false)
    (`Pawn.AddMovementInput` _player_ref (0.0 0.0 1.0) ActionValue_Z false)))

(event `EnhancedInput|/Game/Blueprints/Inputs/IA_Shoot`
  (params (ActionValue :type Boolean) (ElapsedSeconds :type "Float (double-precision)") (TriggeredSeconds :type "Float (double-precision)") (InputAction :type "InputAction Object Reference" :default "/Game/Blueprints/Inputs/IA_Shoot.IA_Shoot"))
  (bind _player_ref (`self.Player_Ref`))
  ; Allows player to shoot with spacebar
  (:`Triggered`
    (if (`self.CanShoot`)
      (set `self.CanShoot` false)
      (`|SpawnActorFromClass` "/Game/Blueprints/BP_Projectile.BP_Projectile_C" (`KismetMathLibrary.MakeTransform` (`SceneComponent.K2_GetComponentLocation` (`/Game/Blueprints/BP_PlayerCharacter.FirePoint` _player_ref)) (`self.K2_GetActorRotation` _player_ref)) "Undefined" "MultiplyWithRoot" null _player_ref null)
      (`KismetSystemLibrary.K2_SetTimerDelegate` (delegate `ResetShootCooldown`) (`self.HammerCooldown`)))))

(event `ResetShootCooldown`
  ; Reset the cooldown for the hammer throw
  (set `self.CanShoot` true))

(fn `UserConstructionScript`)